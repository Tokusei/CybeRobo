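; B_boxtwo is an actor that animates two plane components along the vertical axis when play begins.
; A timeline feeds its Up and Down tracks into the relative Z of Plane and Plane1, keeping X and Y fixed.
; In the Customization level it also destroys its Hit component, then Loop, which is only removed if Hit was valid.
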(event `self.ReceiveBeginPlay`
  (bind _hit (`self.hit`))
  (bind _loop (`self.loop`))
  (`|ExecutionSequence`
    (:`then_0`
      (bind (_direction _up _down) (`Timeline|Timeline_0` :!via `PlayFromStart`)
        (:`Update`
          (`|ExecutionSequence`
            (:`then_0`
              (`SceneComponent.K2_SetRelativeLocation` (`self.Plane`) (`KismetMathLibrary.MakeVector` 205.0 -95.0 _up) false false))
            (:`then_1`
              (`SceneComponent.K2_SetRelativeLocation` (`self.Plane1`) (`KismetMathLibrary.MakeVector` 205.0 -95.0 _down) false false))))))
    (:`then_1`
      (bind _returnvalue (`GameplayStatics.GetCurrentLevelName` true))
      (if (`KismetStringLibrary.EqualEqual_StrStr` _returnvalue "Customization")
        (`/Engine/EditorBlueprintResources/StandardMacros.IsValid` _hit
          (:`Is Valid`
            (`ActorComponent.K2_DestroyComponent` _hit)
            (`/Engine/EditorBlueprintResources/StandardMacros.IsValid` _loop
              (:`Is Valid`
                (`ActorComponent.K2_DestroyComponent` _loop)))))))))

(fn `UserConstructionScript`)