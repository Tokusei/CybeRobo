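; Elevator actor that raises and turns its static mesh when a RoboPawn enters its box trigger or the 9 key is pressed.
; Either trigger sets a Go flag and restarts a timeline, whose Up and Rotation tracks Tick applies as relative Z and yaw.
; A parallel delayed sequence plays the audio component twice during the ride.
; BeginPlay enables input from the first player controller for the key trigger.
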(event `self.ReceiveBeginPlay`
  (`self.EnableInput` (`GameplayStatics.GetPlayerController` 0)))

(event `self.ReceiveTick`
  (params (DeltaSeconds :type "Float (single-precision)"))
  (bind _staticmesh (`self.StaticMesh`))
  (if (`self.go`)
    (`SceneComponent.K2_SetRelativeLocation` _staticmesh (`KismetMathLibrary.MakeVector` 0.0 0.0 (stale `Key|Nine` _up)) false false)
    (`SceneComponent.K2_SetRelativeRotation` _staticmesh (`KismetMathLibrary.MakeRotator` 0.0 0.0 (stale `Key|Nine` _rotation)) false false)))

(event `Key|Nine`
  (params (Key :type "Key Structure"))
  (:`Pressed`
    (set `self.go` true :!label _label)
    (`|ExecutionSequence`
      (:`then_0`
        (bind (_direction _up _rotation) (`Timeline|Timeline_0` :!via `PlayFromStart`)))
      (:`then_1`
        (`KismetSystemLibrary.Delay` 3.5)
        (`AudioComponent.Play` (`self.Audio`) 3.5)
        (`KismetSystemLibrary.Delay` 3.5)
        (`AudioComponent.Play` (`self.Audio`) 3.5)))))

(event `self.Box.OnComponentBeginOverlap`
  (params (OverlappedComponent :type "PrimitiveComponent Object Reference") (OtherActor :type "Actor Object Reference") (OtherComp :type "PrimitiveComponent Object Reference") (OtherBodyIndex :type Integer) (bFromSweep :type Boolean) (SweepResult :type "HitResult Structure (by ref)"))
  (cast `/Game/Core/GameClasses/RoboPawn` OtherActor)
  (goto _label))

(fn `UserConstructionScript`)