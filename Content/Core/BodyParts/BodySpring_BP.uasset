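; BodySpring_BP is a spring body part that animates its Base component's Z scale while the 3 key is held.
; BeginPlay caches the Base's relative transform and enables input for player controller 0.
; Pressing plays a timeline that lerps Z scale from its initial value to a fixed target, keeping other transform values.
; Releasing reverses the timeline from its end, so mid-animation releases jump before returning.
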(event `self.ReceiveBeginPlay`
  (set `self.IntTrans` (`SceneComponent.GetRelativeTransform` (`self.Base`)))
  (`self.EnableInput` (`GameplayStatics.GetPlayerController` 0)))

(event `Key|Three`
  (params (Key :type "Key Structure"))
  (:`Pressed`
    (`self.StartExpand`))
  (:`Released`
    (`self.StopExpand`)))

(event `StartExpand`
  (bind _inttrans (`self.IntTrans`))
  (bind (_direction _1) (`Timeline|Timeline_0` :!via `PlayFromStart` :!label _label)
    (:`Update`
      (`SceneComponent.K2_SetRelativeTransform` (`self.Base`) (`KismetMathLibrary.MakeTransform` (.location _inttrans) (.rotation _inttrans) (`KismetMathLibrary.VLerp` (`KismetMathLibrary.MakeVector` (.x (.scale _inttrans)) (.y (.scale _inttrans)) (.z (.scale _inttrans))) (`KismetMathLibrary.MakeVector` (.x (.scale _inttrans)) (.y (.scale _inttrans)) 0.7) _1)) false false))))

(event `StopExpand`
  (goto _label :!via `ReverseFromEnd`))

(fn `UserConstructionScript`)