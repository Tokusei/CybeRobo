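; Body arm Blueprint that extends and retracts an arm component for a grab motion.
; StartGrab plays a timeline that lerps the Arm's relative location forward along X without sweep, and EndGrab reverses it from the end.
; BeginPlay enables input from the first player controller so a test key can drive both events on press and release.
; A dynamic material setup for the Base is present but never runs.
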(event `StartGrab`
  (bind (_direction _1) (`Timeline|Timeline_0` :!via `PlayFromStart` :!label _label)
    (:`Update`
      (`SceneComponent.K2_SetRelativeLocation` (`self.Arm`) (`KismetMathLibrary.VLerp` (0.0 0.0 0.0) (30.0 0.0 0.0) _1) false false))))

(event `End Grab`
  (goto _label :!via `ReverseFromEnd`))

(event `Key|Four`
  (params (Key :type "Key Structure"))
  ;[1 1 1] test
  (:`Pressed`
    (`self.StartGrab`))
  (:`Released`
    (`self.End Grab`)))

(event `self.ReceiveBeginPlay`
  ;[1 1 1] test
  (`self.EnableInput` (`GameplayStatics.GetPlayerController` 0)))

(fn `UserConstructionScript`)